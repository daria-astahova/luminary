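; BP_PlayerLuminary handles player mouse clicks on BP_PopupObject actors, showing the cursor at BeginPlay.
; A left click deprojects the mouse into a Visibility trace that ignores DisplayCluster root actors, then calls Interact with the hit location.
; The trace end is the scaled mouse direction alone, without the start position added.
; An unconnected TouchOutput debug-print branch never runs.
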(event EventBeginPlay
  (bind _outactors (Actor|GetAllActorsOfClass "/Script/DisplayCluster.DisplayClusterRootActor"))
  (Variables|Default|SetActors%20to%20Ignore _outactors)
  (Variables|/Script/Engine.PlayerController|SetbShowMouseCursor (Game|GetPlayerController 0) true))

(event Collision|EventActorBeginOverlap
  (params (OtherActor :type Actor%20Object%20Reference)))

(event EventTick
  (params (DeltaSeconds :type Float%20%28single-precision%29)))

(event Input|MouseEvents|LeftMouseButton
  (params (Key :type Key%20Structure :default "None"))
  (bind _returnvalue (Game|GetPlayerController 0))
  (bind (_worldlocation _worlddirection) (Game|Player|ConvertMouseLocationToWorldSpace _returnvalue))
  (:Pressed
    (bind _outhit (Collision|LineTraceByChannel _worldlocation (* _worlddirection 99999.0) "TraceTypeQuery1" false (Variables|Default|GetActors%20to%20Ignore) "None"))
    (bind _asbp_popup_object (Utilities|Casting|CastToBP_PopupObject (.HitActor (Collision|BreakHitResult _outhit))))
    (Default|Interact _asbp_popup_object (.Location (Collision|BreakHitResult _outhit)))
    (Development|PrintString "hit")))

(fn ConstructionScript)